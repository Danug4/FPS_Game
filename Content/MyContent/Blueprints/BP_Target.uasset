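; Moving shootable target that oscillates along a direction and is destroyed after taking enough hits.
; Tick offsets it by normalized Direction times Speed, without delta-time scaling, while a looping timer reverses Direction every MovementDuration.
; Hit decrements HitPoints; on death it spawns a Niagara effect chosen by TargetType colour, plays a big explosion and destroys itself.
; Non-lethal hits play a small explosion at world origin rather than HitLocation.
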(event Custom|Event_FlipDirection
  ;[0.05313 0.06262 0.15 0.5] Flip Direction
  (Variables|Default|SetDirection (* -1.0 (Variables|Default|GetDirection))))

(event EventBeginPlay
  ;[0.05313 0.06262 0.15 0.5] Flip Direction
  (Utilities|Time|SetTimerbyEvent (delegate Custom|Event_FlipDirection) (Variables|Default|GetMovementDuration) true))

(event EventTick
  (params (DeltaSeconds :type Float%20%28single-precision%29))
  ;[0.15 0.06311 0.02031 0.5] Target Movement
  (Transformation|AddActorWorldOffset (* (Math|Vector|Normalize (Variables|Default|GetDirection)) (Variables|Default|GetSpeed))))

(event Collision|EventHit
  (params (MyComp :type Primitive%20Component%20Object%20Reference) (Other :type Actor%20Object%20Reference) (OtherComp :type Primitive%20Component%20Object%20Reference) (bSelfMoved :type Boolean) (HitLocation :type Vector :default "0, 0, 0") (HitNormal :type Vector :default "0, 0, 0") (NormalImpulse :type Vector :default "0, 0, 0") (Hit :type Hit%20Result%20Structure%20%28by%20ref%29))
  ;[0.15 0.15 0.15 0.5] Target Hit
  (Variables|Default|SetHitPoints (- (Variables|Default|GetHitPoints) 1))
  ;[0.15 0.15 0.15 0.5] Check If target is "dead"
  (if (<= (Variables|Default|GetHitPoints) 0)
    ;[0.3802 0 0 0.5] If Red Target
    (if (== (Variables|Default|GetTargetType) 0)
      ;[0.15 0.15 0.15 0.5] Play Particle Effect depending on type
      (Niagara|SpawnSystematLocation "/Game/MyContent/FX/PE_Target_Hit_Red.PE_Target_Hit_Red" HitLocation)
      (else
        ;[0.05186 0.15 0.01697 0.5] If Green Target
        (if (== (Variables|Default|GetTargetType) 1)
          (Niagara|SpawnSystematLocation "/Game/MyContent/FX/PE_Target_Hit_Green.PE_Target_Hit_Green" HitLocation)
          (else
            ;[0.02552 0.032 0.15 0.5] If Blue Target
            (if (== (Variables|Default|GetTargetType) 2)
              (Niagara|SpawnSystematLocation "/Game/MyContent/FX/PE_Target_Hit_Blue.PE_Target_Hit_Blue" HitLocation)
              (else
                (Niagara|SpawnSystematLocation "/Game/MyContent/FX/PE_Target_Hit.PE_Target_Hit" HitLocation)))))))
    (Audio|SpawnSoundatLocation "/Game/MyContent/Audio/MP3_Explosion_Big.MP3_Explosion_Big" HitLocation "0, 0, 0" 1.0 1.0 0.0 0 0)
    (Actor|DestroyActor)
    (else
      (Audio|SpawnSoundatLocation "/Game/MyContent/Audio/MP3_Explosions_Small.MP3_Explosions_Small" "0, 0, 0" "0, 0, 0" 1.0 1.0 0.0 0 0))))

(fn ConstructionScript)