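; BP_Tree is an actor that serves as an ammunition pickup point for the first-person player.
; On BeginPlay it caches the player character as BP_FirstPersonCharacter and clears that character's MayGrabAmmo flag.
; Overlap begin and end events toggle the flag for that player only, printing an "e" key prompt on entry.
; The tree only sets permission and contains no input handling or ammo-granting logic.
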(event EventBeginPlay
  ;[0.15 0.15 0.15 0.5] Find Player Character
  (bind _asbp_first_person_character (Utilities|Casting|CastToBP_FirstPersonCharacter (Game|GetPlayerCharacter 0)))
  (bind _output_get (Variables|Default|SetPlayer _asbp_first_person_character))
  (Variables|/Game/StarterContent/FirstPerson/Blueprints/BP_FirstPersonCharacter.BP_FirstPersonCharacter_C|SetMayGrabAmmo _output_get false))

(event Collision|EventActorEndOverlap
  (params (OtherActor :type Actor%20Object%20Reference))
  ;[0.15 0.15 0.15 0.5] If Player Leaves Tree: Turn off ability to add ammo
  (if (== OtherActor (Variables|Default|GetPlayer))
    (Variables|/Game/StarterContent/FirstPerson/Blueprints/BP_FirstPersonCharacter.BP_FirstPersonCharacter_C|SetMayGrabAmmo (Variables|Default|GetPlayer) false)))

(event Collision|EventActorBeginOverlap
  (params (OtherActor :type Actor%20Object%20Reference))
  ;[0.15 0.15 0.15 0.5] If in range of tree: Allow player to grab ammo
  (if (== OtherActor (Variables|Default|GetPlayer))
    (Variables|/Game/StarterContent/FirstPerson/Blueprints/BP_FirstPersonCharacter.BP_FirstPersonCharacter_C|SetMayGrabAmmo (Variables|Default|GetPlayer) true)
    (Development|PrintString "Press \"e\" to grab ammunition")))

(fn ConstructionScript)