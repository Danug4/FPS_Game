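; Stealth security camera that sweeps between two rotations and catches the first-person player in its line of sight.
; A self-repeating event flip-flops between start and end rotations, moving the mesh over time and pausing before the next swing.
; Every tick, a debug-drawn forward line trace checks for the player pawn, then flags it caught and disables input.
; The delayed StealthMap reload is disconnected and never runs.
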(event Custom|Move_Camera
  ;[0.15 0.15 0.15 0.5] Camera Movement
  (Utilities|FlowControl|FlipFlop
    (:A
      (Variables|Default|SetCurrentRotation (Variables|Default|GetStartRotation)))
    (:B
      (Variables|Default|SetCurrentRotation (Variables|Default|GetEndRotation))))
  (Components|MoveComponentTo (Variables|Default|GetSM_SecurityCamera) "0, 0, 0" (Math|Rotator|MakeRotator (.x (Variables|Default|GetCurrentRotation)) (.y (Variables|Default|GetCurrentRotation)) (.z (Variables|Default|GetCurrentRotation))) false false (Variables|Default|GetSpeed) false)
  (Utilities|FlowControl|Delay (Variables|Default|GetDelay))
  (CallFunction|MoveCamera))

(event Custom|Detect
  (bind _bp_first_person_character (Variables|Default|GetBP%20First%20Person%20Character))
  (bind _sm_linetrace (Variables|Default|GetSM_LineTrace))
  (bind _returnvalue (Transformation|GetWorldLocation _sm_linetrace))
  ;[0.15 0.15 0.15 0.5] Camera Detection
  (bind _outhit (Collision|LineTraceForObjects _returnvalue (+ _returnvalue (* (Math|Vector|GetForwardVector (Transformation|GetWorldRotation _sm_linetrace)) (Variables|Default|GetDetectDistance))) (Utilities|Array|MakeArray "ObjectTypeQuery3") false 0 "ForOneFrame"))
  (if (== (.HitActor (Collision|BreakHitResult _outhit)) _bp_first_person_character)
    (Variables|/Game/StarterContent/FirstPerson/Blueprints/BP_FirstPersonCharacter.BP_FirstPersonCharacter_C|SetIs_Caught _bp_first_person_character true)
    ;[0.15 0.15 0.15 0.5] Disable Input and Reload Level
    (Input|DisableInput (Variables|Default|GetBP%20First%20Person%20Character) (Game|GetPlayerController 0))))

(event EventBeginPlay
  (CallFunction|MoveCamera)
  (bind _asbp_first_person_character (Utilities|Casting|CastToBP_FirstPersonCharacter (Game|GetPlayerCharacter 0)))
  (Variables|Default|SetBP%20First%20Person%20Character _asbp_first_person_character))

(event EventTick
  (params (DeltaSeconds :type Float%20%28single-precision%29))
  (CallFunction|Detect))

(fn ConstructionScript)